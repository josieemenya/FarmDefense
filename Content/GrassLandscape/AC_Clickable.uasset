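; Actor component that makes its owning actor clickable, toggling the material on that actor's static mesh.
; On BeginPlay it binds to the owner's OnClicked event and caches the owner's StaticMeshComponent.
; Each click flips a boolean and swaps material slot 0 between the Weclick and Alpha_Body_MAT materials when a mesh is found.
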(event Custom|Click
  (params (TouchedActor :type Actor%20Object%20Reference) (ButtonPressed :type Key%20Structure :default "None"))
  (bind _staticmeshref (Variables|Default|GetStaticMeshRef))
  (bind _output_get (Variables|Default|SetisClicked (not (Variables|Default|GetisClicked))))
  (Utilities|IsValid _staticmeshref
    (:Is%20Valid
      (if _output_get
        (Rendering|Material|SetMaterial _staticmeshref 0 (Variables|Default|Getweclick))
        (else
          (Rendering|Material|SetMaterial _staticmeshref 0 "/Game/GameContent/Farmer/Animations/Alpha_Body_MAT.Alpha_Body_MAT"))))))

(event EventBeginPlay
  (bind _returnvalue (Components|GetOwner))
  (bind _returnvalue_2 (Actor|GetComponentbyClass _returnvalue "/Script/Engine.StaticMeshComponent"))
  (EventDispatchers|BindEventtoOnClicked _returnvalue (delegate Custom|Click))
  (Utilities|IsValid _returnvalue_2
    (:Is%20Valid
      (Variables|Default|SetStaticMeshRef _returnvalue_2))))